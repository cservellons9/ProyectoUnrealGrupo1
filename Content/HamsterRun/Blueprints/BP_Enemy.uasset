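; BP_Enemy is an enemy actor for HamsterRun with simple health and attack damage.
; It damages the runner character on overlap, and its own health starts at maximum, drops on any damage and destroys the actor at zero.
; A separate Attacktrace function fires a debug-drawn forward line trace that damages whatever it hits, though nothing in this Blueprint calls it.
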(event EventTick
  (params (DeltaSeconds :type Float%20%28single-precision%29)))

(event EventBeginPlay
  (Variables|Default|Setcurrenthealth (Variables|Default|Getmaxhealth)))

(event Game|Damage|EventAnyDamage
  (params (Damage :type Float%20%28single-precision%29) (DamageType :type Damage%20Type%20Object%20Reference) (InstigatedBy :type Controller%20Object%20Reference) (DamageCauser :type Actor%20Object%20Reference))
  (bind _output_get (Variables|Default|Setcurrenthealth (- (Variables|Default|Getcurrenthealth) Damage)))
  (if (<= _output_get 0.0)
    (Actor|DestroyActor)
    (else
      (Development|PrintString "Enemy hit"))))

(event Collision|EventActorBeginOverlap
  (params (OtherActor :type Actor%20Object%20Reference))
  (Utilities|Casting|CastToBP_runnerCharacter OtherActor)
  (Game|Damage|ApplyDamage OtherActor (Variables|Default|Getattackdamage) 0 self)
  (Development|PrintString "Player Hit!" true true "(R=1.000000,G=0.000000,B=0.000000,A=1.000000)"))

(fn ConstructionScript)

(fn Attacktrace
  (bind _scene (Variables|Default|GetScene))
  (bind _returnvalue (Transformation|GetWorldLocation _scene))
  (bind (_outhit _returnvalue_2) (Collision|LineTraceByChannel _returnvalue (+ _returnvalue (* (Math|Vector|GetForwardVector _scene) 1e+03)) "TraceTypeQuery3" false 0 "ForOneFrame"))
  (if _returnvalue_2
    (Development|PrintString (Utilities|GetObjectName (.HitActor (Collision|BreakHitResult _outhit))))
    (Game|Damage|ApplyDamage (.HitActor (Collision|BreakHitResult _outhit)) (Variables|Default|Getattackdamage) 0 self)))